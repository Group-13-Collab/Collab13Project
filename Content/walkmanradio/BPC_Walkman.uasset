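; Walkman component that lets the player control music playback through the character's Audio component using Enhanced Input.
; The first IA_Radio press starts playback; a short press toggles pause on release.
; Holding it while on fires the audio's SkipSong trigger parameter, gated by a DoOnce that resets after a retriggerable delay.
; IA_Radio_vol steps the volume multiplier within a clamped range while on, with debug prints reporting changes.
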(event Input|EnhancedActionEvents|EnhancedInputActionIA_Radio
  (params (ActionValue :type Boolean) (ElapsedSeconds :type Float%20%28double-precision%29) (TriggeredSeconds :type Float%20%28double-precision%29) (InputAction :type Input%20Action%20Object%20Reference :default "/Game/Inputs/PlayerInputs/IA_Radio.IA_Radio"))
  (bind _returnvalue (>= TriggeredSeconds 2.0))
  (bind _audio (Variables|Default|GetAudio))
  (:Triggered
    ;[0.15 0.15 0.15 0.5] Manualskip song
    (if (and (Variables|Default|GetIsOn?) _returnvalue)
      (Utilities|FlowControl|DoOnce false :!label _label
        (:Completed
          (Development|PrintString "Skipping Song" true true "(R=1.000000,G=0.000000,B=0.716799,A=1.000000)")
          (Class|AudioParameterControllerInterface|SetTriggerParameter (Variables|Default|GetAudio) "SkipSong")
          (Development|PrintString "Song has been skipped")
          (Utilities|FlowControl|RetriggerableDelay 3.0)
          (goto _label Reset)))))
  (:Started
    ;[0.15 0.15 0.15 0.5] To turn on the walkman
    (Utilities|FlowControl|DoOnce false
      (:Completed
        (Audio|Components|Audio|Play (Variables|Default|GetAudio) 0.0))))
  (:Completed
    ;[0.15 0.15 0.15 0.5] Pause/Unpause
    (if (Variables|Default|GetIsOn?)
      (if (not _returnvalue)
        (Variables|Default|SetIsOn? false)
        (Class|AudioComponent|SetPaused _audio true)
        (Development|PrintString "Walkman OFF" true true "(R=1.000000,G=0.070265,B=0.000000,A=1.000000)"))
      (else
        (Variables|Default|SetIsOn? true)
        (Class|AudioComponent|SetPaused _audio false)
        (Development|PrintString "Walkman ON")))))

(event Input|EnhancedActionEvents|EnhancedInputActionIA_Radio_vol
  (params (ActionValue :type Float%20%28double-precision%29) (ElapsedSeconds :type Float%20%28double-precision%29) (TriggeredSeconds :type Float%20%28double-precision%29) (InputAction :type Input%20Action%20Object%20Reference :default "/Game/Inputs/PlayerInputs/IA_Radio_vol.IA_Radio_vol"))
  (bind _audio (Variables|Default|GetAudio))
  ;[0.15 0.15 0.15 0.5] Volume
  (:Started
    (if (Variables|Default|GetIsOn?)
      (if (== ActionValue 1.0)
        (bind _returnvalue (CallFunction|WalkmanVolume _audio 0.25))
        (Development|PrintString (Utilities|String|Append "Current Level: " (Utilities|String|ToString(Float) _returnvalue)))
        (else
          (bind _returnvalue_2 (CallFunction|WalkmanVolume _audio -0.25))
          (Development|PrintString (Utilities|String|Append "Current Level: " (Utilities|String|ToString(Float) _returnvalue_2))))))))

(event EventBeginPlay
  ;[0.001584 0.15 0.1225 0.5] BeginPlay
  (Variables|Default|SetAudio (Variables|/Game/Player/BP_PlayerCharacter.BP_PlayerCharacter_C|GetAudio (CallFunction|GetPlayerCharacter))))

(fn WalkmanVolume
  (params (Target :type Audio%20Component%20Object%20Reference) (B :type Float%20%28double-precision%29))
  (bind _volumemultiplier (Variables|/Script/Engine.AudioComponent|GetVolumeMultiplier Target))
  (bind _returnvalue (+ _volumemultiplier B))
  (bind _returnvalue_2 (Math|Float|Clamp(Float) _returnvalue 0.1))
  (Audio|Components|Audio|SetVolumeMultiplier Target _returnvalue_2 :!class /Script/Engine.AudioComponent)
  (return _returnvalue_2))