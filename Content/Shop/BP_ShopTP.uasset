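; BP_ShopTP is an interactable shop entrance that teleports the player to the shop.
; Its InteractedWith function plays a door-open sound, then moves player 0's character to the root location of the BP_ShopLocation actor found in the level.
; The move is an unswept teleport, and the function always returns false.
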(event EventBeginPlay
  (|CallParentFunction) ; This node is disabled and will not be called.\nDrag off pins to build functionality.
)

(event Collision|EventActorBeginOverlap
  (params (OtherActor :type Actor%20Object%20Reference)))

(event EventTick
  (params (DeltaSeconds :type Float%20%28single-precision%29)))

(fn ConstructionScript
  (|CallParentFunction))

(fn Interactedwith
  (Audio|PlaySound2D "/Game/Audio/SFX/Metasound/MS_Door_Open.MS_Door_Open" 1.0 1.0 0.0 0 0)
  (bind _returnvalue (Actor|GetActorOfClass "/Game/Shop/BP_ShopLocation.BP_ShopLocation_C"))
  (Transformation|SetActorLocation (Game|GetPlayerCharacter 0) (Transformation|GetWorldLocation (Variables|/Game/Shop/BP_ShopLocation.BP_ShopLocation_C|GetDefaultSceneRoot _returnvalue)) false true)
  (return false))