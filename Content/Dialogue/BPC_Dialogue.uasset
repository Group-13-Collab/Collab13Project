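; Dialogue component for NPCs that shows quest-giving or quest-completed lines matching the reputation mood: Happy, Neutral or Unhappy.
; InteractWith adds a dialogue canvas widget, plays the player's seagull greeting animation and fills the dialogue box from per-NPC string arrays.
; On completion it refreshes the owner's reputation from the player's points; otherwise it uses the passed-in type.
; StartDialogue is empty and GetReputation always returns Happy.
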(event EventBeginPlay)

(fn StartDialogue)

(fn GetReputation
  (return "NewEnumerator0"))

(fn Interactwith
  (params (IsQuestCompleted? :type Boolean) (ReputationType :type E_Reputation%20Enum :default "NewEnumerator0"))
  (bind _returnvalue (Components|GetOwner))
  (bind _returnvalue_2 (UserInterface|CreateWidget "/Game/Dialogue/WBP_DialogueCanvas.WBP_DialogueCanvas_C"))
  (UserInterface|Viewport|AddtoViewport _returnvalue_2 0)
  ;[0.15 0.15 0.15 0.5] temp fix?
  (Components|Animation|PlayAnimation (Variables|/Script/Engine.Character|GetMesh (CallFunction|GetPlayerCharacter)) "/Game/Animation/SeagullAnimations/SeagullGreeting.SeagullGreeting" false)
  (if IsQuestCompleted? ; is quest complete?
    (Components|Animation|PlayAnimation (Variables|/Script/Engine.Character|GetMesh (CallFunction|GetPlayerCharacter)) "/Game/Animation/SeagullAnimations/SeagullGreeting.SeagullGreeting" false)
    (bind _points (Class|BPIPlayerInformation|GetCalculatedReputationPoints(Message) (Game|GetPlayerCharacter 0)))
    (Class|IInteractionInterface|UpdateReputationPoints(Message) _returnvalue _points)
    (bind _reputationtype (Class|IInteractionInterface|GetReputation(Message) _returnvalue))
    (switch Utilities|FlowControl|Switch|SwitchonE_Reputation _reputationtype
      (:NewEnumerator0
        (Default|FillDialogueArray (Variables|/Game/Dialogue/WBP_DialogueCanvas.WBP_DialogueCanvas_C|GetWBP_DialogueBox _returnvalue_2) (Variables|Default|GetCompletedTask_Happy) self IsQuestCompleted?) ; Sets the dialogue in the widget blueprint
      )
      (:NewEnumerator1
        (Default|FillDialogueArray (Variables|/Game/Dialogue/WBP_DialogueCanvas.WBP_DialogueCanvas_C|GetWBP_DialogueBox _returnvalue_2) (Variables|Default|GetCompletedTask_Neutral) self IsQuestCompleted?) ; Sets the dialogue in the widget blueprint
      )
      (:NewEnumerator2
        (Default|FillDialogueArray (Variables|/Game/Dialogue/WBP_DialogueCanvas.WBP_DialogueCanvas_C|GetWBP_DialogueBox _returnvalue_2) (Variables|Default|GetCompletedTask_Unhappy) self IsQuestCompleted?) ; Sets the dialogue in the widget blueprint
      ))
    (else
      (switch Utilities|FlowControl|Switch|SwitchonE_Reputation ReputationType
        (:NewEnumerator0
          (Default|FillDialogueArray (Variables|/Game/Dialogue/WBP_DialogueCanvas.WBP_DialogueCanvas_C|GetWBP_DialogueBox _returnvalue_2) (Variables|Default|GetGivingTask_Happy) self IsQuestCompleted?) ; Sets the dialogue in the widget blueprint
        )
        (:NewEnumerator1
          (Default|FillDialogueArray (Variables|/Game/Dialogue/WBP_DialogueCanvas.WBP_DialogueCanvas_C|GetWBP_DialogueBox _returnvalue_2) (Variables|Default|GetGivingTask_Neutral) self IsQuestCompleted?) ; Sets the dialogue in the widget blueprint
        )
        (:NewEnumerator2
          (Default|FillDialogueArray (Variables|/Game/Dialogue/WBP_DialogueCanvas.WBP_DialogueCanvas_C|GetWBP_DialogueBox _returnvalue_2) (Variables|Default|GetGivingTask_Unhappy) self IsQuestCompleted?) ; Sets the dialogue in the widget blueprint
        )))))