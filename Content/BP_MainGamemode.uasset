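; Main game mode that tracks overall quest progress and times quests.
; Tick watches the quest counter and, at the completion threshold, flags all quests complete and adds the end quest to the quest log on every tick, with no one-shot guard.
; A very long one-shot timer serves as a stopwatch: functions read or stop it to return elapsed time, and expiry sets a huge sentinel value.
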(event Custom|QuestTimer
  (Variables|Default|SetElapsedTime 9999999.0))

(event EventBeginPlay)

(event EventTick
  (params (DeltaSeconds :type Float%20%28single-precision%29))
  (if (>= (Variables|Default|GetQuestCounter) 13)
    (Variables|Default|SetAllQuestsComplete true)
    (Default|AddNewQuest (Variables|Default|GetQuestLog) "endquest")))

(event EventStartQuestTimer
  (bind _returnvalue (Utilities|Time|SetTimerbyEvent (delegate Custom|QuestTimer) 1e+05))
  (Variables|Default|SetQuestTime _returnvalue))

(fn ConstructionScript)

(fn GetQuestTimerElapsedTime
  (bind _output_get (Variables|Default|SetElapsedTime (Class|KismetSystemLibrary|GetTimerElapsedTimeHandle (Variables|Default|GetQuestTime))))
  (return _output_get))

(fn StopQuestTimer
  (bind _output_get (Variables|Default|SetElapsedTime (Class|KismetSystemLibrary|GetTimerElapsedTimeHandle (Variables|Default|GetQuestTime))))
  (Utilities|Time|ClearandInvalidateTimerbyHandle (Variables|Default|GetQuestTime))
  (return _output_get))