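; BP_ShopShelf is an interactable shop shelf that the player empties one item at a time.
; A sphere overlap flags when the player is near and registers the shelf as the player character's NearestShelf, which is not cleared on exit.
; While the player is near, ItemInteract calls DestroyItem on the current ShopItems entry and advances the index, printing a message when no valid item remains.
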(event OnComponentBeginOverlap(Sphere)
  (params (OverlappedComponent :type Primitive%20Component%20Object%20Reference) (OtherActor :type Actor%20Object%20Reference) (OtherComp :type Primitive%20Component%20Object%20Reference) (OtherBodyIndex :type Integer) (bFromSweep :type Boolean) (SweepResult :type Hit%20Result%20Structure%20%28by%20ref%29))
  (if (== OtherActor (Variables|Default|GetAs%20BP%20Player%20Character))
    (Variables|/Game/Player/BP_PlayerCharacter.BP_PlayerCharacter_C|SetNearestShelf (Variables|Default|GetAs%20BP%20Player%20Character) self)
    (Variables|Default|SetIsNearShelf true)))

(event OnComponentEndOverlap(Sphere)
  (params (OverlappedComponent :type Primitive%20Component%20Object%20Reference) (OtherActor :type Actor%20Object%20Reference) (OtherComp :type Primitive%20Component%20Object%20Reference) (OtherBodyIndex :type Integer))
  (if (== OtherActor (Variables|Default|GetAs%20BP%20Player%20Character))
    (Variables|Default|SetIsNearShelf false)))

(event Custom|ItemInteract
  (bind _shopitems (Variables|Default|GetShopItems))
  (bind _itemsindex (Variables|Default|GetItemsIndex))
  (bind _output (Utilities|Array|Get(acopy) _shopitems _itemsindex))
  (if (Variables|Default|GetIsNearShelf)
    (Utilities|IsValid _output
      (:Is%20Valid
        (Default|DestroyItem _output)
        (Math|Integer|IncrementInt (Variables|Default|GetItemsIndex)))
      (:Is%20Not%20Valid
        (Development|PrintString "No more items in the shelf")))))

(event EventBeginPlay
  (bind _asbp_player_character (Utilities|Casting|CastToBP_PlayerCharacter (Game|Player|GetPlayerPawn 0)))
  (Variables|Default|SetAs%20BP%20Player%20Character _asbp_player_character))

(fn ConstructionScript)