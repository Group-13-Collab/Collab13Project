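; Manager Blueprint that applies consumed upgrade pickups to the player's BPCUpgrades component.
; On BeginPlay it caches that component and binds to OnUpgradeConsumed on every BP_UpgradeItem_Base in the level.
; The handler switches on upgrade type: speed unlocks skates once and sets skate speed, reputation and money pass multiplied values to boost functions, and temp boosts add a charge with a reward message.
; GetReputation and InteractWith are placeholder stubs.
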(event Custom|CustomEvent
  (params (UpgradeInfo :type DS%20Upgrade%20Info%20Structure))
  (bind _upgrade_reference (Variables|Default|GetUpgrade%20Reference))
  (bind _upgrade_reference_2 (Variables|Default|GetUpgrade%20Reference))
  (bind _upgrade_reference_3 (Variables|Default|GetUpgrade%20Reference))
  (bind _upgrade_reference_4 (Variables|Default|GetUpgrade%20Reference))
  ;[0.15 0.15 0.15 0.5] Perma Upgrades When Consumed. Could be better
  (bind _output_get (Variables|Main|SetUpgradeData UpgradeInfo))
  (switch Utilities|FlowControl|Switch|SwitchonE_Upgrade (Utilities|Struct|BreakDS_UpgradeInfo _output_get)
    (:NewEnumerator0
      (Utilities|FlowControl|Sequence
        (:then_0
          (Utilities|FlowControl|DoOnce false
            (:Completed
              (Variables|/Game/Interactables/Upgrades/BPC_Upgrades.BPC_Upgrades_C|SetHasSkates? _upgrade_reference_4 true))))
        (:then_1
          (bind _output_get_2 (Variables|/Game/Interactables/Upgrades/BPC_Upgrades.BPC_Upgrades_C|SetSkateSpeed _upgrade_reference_4 (Utilities|Struct|BreakDS_UpgradeInfo (Variables|Main|GetUpgradeData))))
          (Development|PrintString (Utilities|String|Append "Skate  Speed: " (Utilities|String|ToString(Float) _output_get_2))))))
    (:NewEnumerator1
      (bind _output_get_3 (Variables|/Game/Interactables/Upgrades/BPC_Upgrades.BPC_Upgrades_C|SetUpgradeInfo _upgrade_reference_3 (Utilities|Struct|MakeDS_UpgradeInfo (* (Variables|Default|GetBaseMulti) (Utilities|Struct|BreakDS_UpgradeInfo (Variables|Main|GetUpgradeData))))))
      (Default|RepBoost _upgrade_reference_3 _output_get_3))
    (:NewEnumerator3
      (bind _output_get_4 (Variables|/Game/Interactables/Upgrades/BPC_Upgrades.BPC_Upgrades_C|SetUpgradeInfo _upgrade_reference_2 (Utilities|Struct|MakeDS_UpgradeInfo (* 1.0 (Utilities|Struct|BreakDS_UpgradeInfo (Variables|Main|GetUpgradeData))))))
      (Default|MoneyBoost _upgrade_reference_2 _output_get_4))
    (:NewEnumerator2
      (Utilities|IsValid _upgrade_reference
        (:Is%20Valid
          (Default|AddTempAmount _upgrade_reference)
          (Class|BPIRewardBoost|RewardGet(Message) (Variables|/Game/Player/BP_PlayerCharacter.BP_PlayerCharacter_C|GetBPC_Upgrades (CallFunction|GetPlayerCharacter))))))))

(event EventBeginPlay
  ;[0.15 0.15 0.15 0.5] Beginplay. Finds all the actors attached to the array (may change to of class)
  (bind _output_get (Variables|Main|SetPlayer%20Character (CallFunction|GetPlayerCharacter)))
  (Variables|Default|SetUpgrade%20Reference (Variables|/Game/Player/BP_PlayerCharacter.BP_PlayerCharacter_C|GetBPC_Upgrades _output_get))
  (bind _output_get_2 (Variables|Main|SetCharacter%20Movement (Variables|/Script/Engine.Character|GetCharacterMovement _output_get)))
  (Variables|Default|SetCurrentMaxSpeed (Variables|/Script/Engine.CharacterMovementComponent|GetMaxWalkSpeed _output_get_2))
  (bind _outactors (Actor|GetAllActorsOfClass "/Game/Interactables/Upgrades/BP_UpgradeItem_Base.BP_UpgradeItem_Base_C"))
  (for _array_element _outactors
    (Utilities|IsValid _array_element
      (:Is%20Valid
        (EventDispatchers|BindEventtoOnUpgradeConsumed _array_element (EventDispatchers|CreateEvent :!event Custom|CustomEvent))))))

(fn ConstructionScript)

(fn GetReputation
  (return "NewEnumerator0"))

(fn Interactwith
  (params (IsQuestCompleted? :type Boolean) (ReputationType :type E_Reputation%20Enum :default "NewEnumerator0"))
  (return ""))