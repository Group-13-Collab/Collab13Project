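; Skates upgrade component that lets the player switch a movement speed boost on and off with the R key.
; ToggleSkates only works when HasSkates is true and tracks the active state in SkatesCurrentlyOn.
; Turning skates on multiplies the player character's MaxWalkSpeed by SkateSpeed, while turning them off resets it to a hard-coded default instead of the previous value.
; Debug strings report each outcome.
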(event Input|KeyboardEvents|R
  (params (Key :type Key%20Structure :default "None"))
  (:Pressed
    (CallFunction|ToggleSkates)))

(fn ToggleSkates
  (bind _playercharacter (CallFunction|GetPlayerCharacter))
  (bind _skatespeed (Variables|Default|GetSkateSpeed))
  (bind _charactermovement (Variables|/Script/Engine.Character|GetCharacterMovement _playercharacter))
  (if (Variables|Default|GetHasSkates?)
    (if (Variables|Default|GetSkatesCurrentlyOn?)
      (Variables|Default|SetSkatesCurrentlyOn? false)
      (Variables|/Script/Engine.CharacterMovementComponent|SetMaxWalkSpeed (Variables|/Script/Engine.Character|GetCharacterMovement (CallFunction|GetPlayerCharacter)) 6e+02)
      (Development|PrintString "skates off" true true "(R=1.000000,G=0.000000,B=0.004870,A=1.000000)")
      (else
        (Variables|Default|SetSkatesCurrentlyOn? true)
        (bind _output_get (Variables|/Script/Engine.CharacterMovementComponent|SetMaxWalkSpeed _charactermovement (* (Variables|/Script/Engine.CharacterMovementComponent|GetMaxWalkSpeed _charactermovement) _skatespeed)))
        (Development|PrintString "Skates on" true true "(R=1.000000,G=0.000000,B=0.633330,A=1.000000)")
        (Development|PrintString (Utilities|String|Append "Current multi: " (Utilities|String|ToString(Float) _skatespeed) " 
Current speed: " (Utilities|String|ToString(Float) _output_get)) true true "(R=1.000000,G=0.000000,B=0.633330,A=1.000000)")))
    (else
      (Development|PrintString "No skaes")
      (return))))