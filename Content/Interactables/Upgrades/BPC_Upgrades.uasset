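; Player upgrade component providing roller skates, stockpiled temporary speed boosts, and reputation and money upgrade struct helpers.
; R toggles owned skates, attaching them to foot sockets once, then switching visibility, capsule height and walk speed.
; C spends a boost charge to double speed and start a timer, with ResetSpeed halving it.
; Skates and boosts share a tracked current speed, with saved base and boosted values restored on skate removal.
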(event EventBeginPlay
  (bind _output_get (Variables|Default|SetCharacter%20Movement (Variables|/Script/Engine.Character|GetCharacterMovement (CallFunction|GetPlayerCharacter))))
  (bind _output_get_2 (Variables|Default|SetBaseSpeed (Variables|/Script/Engine.CharacterMovementComponent|GetMaxWalkSpeed _output_get)))
  (Variables|Default|SetCurrentPlayerSpeed _output_get_2))

(event Input|KeyboardEvents|C
  (params (Key :type Key%20Structure :default "None"))
  (:Pressed
    (CallFunction|UseTempBoost)))

(event Input|KeyboardEvents|R
  (params (Key :type Key%20Structure :default "None"))
  (:Pressed
    (CallFunction|ToggleSkates)))

(fn ToggleSkates
  (bind _playercharacter (CallFunction|GetPlayerCharacter))
  (bind _mesh (Variables|/Script/Engine.Character|GetMesh _playercharacter))
  (if (Variables|Default|GetHasSkates?)
    (if (Variables|Default|GetSkatesCurrentlyOn?)
      (Variables|Default|SetSkatesCurrentlyOn? false)
      (CallFunction|TakeSkatesOff)
      (else
        (Variables|Default|SetSkatesCurrentlyOn? true)
        (Utilities|FlowControl|Sequence
          (:then_0
            (Utilities|FlowControl|DoOnce false
              (:Completed
                ;[0.15 0.15 0.15 0.5] Attaching the skates to the player's feet so when the player moves, the skates move with the feet
                (Transformation|AttachComponentToComponent (Variables|/Game/Player/BP_PlayerCharacter.BP_PlayerCharacter_C|GetRollerSkatesL _playercharacter) _mesh "L_foot_int" "SnapToTarget" "KeepWorld" "KeepRelative" true)
                (Transformation|AttachComponentToComponent (Variables|/Game/Player/BP_PlayerCharacter.BP_PlayerCharacter_C|GetRollerSkatesR _playercharacter) _mesh "R_foot_int" "SnapToTarget" "KeepWorld" "KeepRelative" true))))
          (:then_1
            (CallFunction|PuttingSkateson)))))
    (else
      (return))))

(fn TempBoost
  (Variables|Default|SetHasBoostOn? true)
  (bind _output_get (Variables|/Script/Engine.CharacterMovementComponent|SetMaxWalkSpeed (Variables|Default|GetCharacter%20Movement) (* (Variables|Default|GetCurrentPlayerSpeed) 2.0)))
  (bind _output_get_2 (Variables|Default|SetCurrentPlayerSpeed _output_get))
  (bind _output_get_3 (Variables|Default|SetBoostedSpeed _output_get_2))
  (Development|PrintString (Utilities|String|Append "Temp Speed: " (Utilities|String|ToString(Float) _output_get_3)) true true "(R=1.000000,G=0.000000,B=0.088880,A=1.000000)")
  (Utilities|Time|SetTimerbyEvent (EventDispatchers|CreateEvent :!event ResetSpeed) 4.0))

(fn ResetSpeed
  (Variables|Default|SetHasBoostOn? false)
  (bind _output_get (Variables|/Script/Engine.CharacterMovementComponent|SetMaxWalkSpeed (Variables|/Script/Engine.Character|GetCharacterMovement (CallFunction|GetPlayerCharacter)) (/ (Variables|Default|GetCurrentPlayerSpeed) 2.0)))
  (Development|PrintString (Utilities|String|Append "Boost wore off" " 
Set current speed to: " (Utilities|String|ToString(Float) _output_get)) true true "(R=1.000000,G=0.000209,B=0.055665,A=1.000000)"))

(fn UseTempBoost
  (if (>= (Variables|Default|GetTempBoostAmount) 1)
    (Development|PrintString "USED" true true "(R=0.534285,G=0.027915,B=1.000000,A=1.000000)")
    (Variables|Default|SetTempBoostAmount (- (Variables|Default|GetTempBoostAmount) 1))
    (CallFunction|TempBoost)
    (else
      (Development|PrintString "CANNOT USE" true true "(R=1.000000,G=0.027465,B=0.000000,A=1.000000)"))))

(fn AddTempAmount
  (bind _output_get (Variables|Default|SetTempBoostAmount (+ (Variables|Default|GetTempBoostAmount) 1)))
  (Development|PrintString (Utilities|String|Append "Picked up!" "YOU CURRENTLY HAVE : " (Utilities|String|ToString(Integer) _output_get)) true true "(R=1.000000,G=0.669749,B=0.000000,A=1.000000)"))

(fn RepBoost
  (params (DS%20Upgrades1 :type DS%20Upgrade%20Info%20Structure))
  (bind _structout (Utilities|Struct|SetmembersinDS_UpgradeInfo DS%20Upgrades1))
  (Development|PrintString (Utilities|String|ToString(Float) (Utilities|Struct|BreakDS_UpgradeInfo _structout)) true true "(R=0.129585,G=1.000000,B=0.000000,A=1.000000)")
  (return _structout))

(fn MoneyBoost
  (params (NewParam :type DS%20Upgrade%20Info%20Structure))
  (bind _structout (Utilities|Struct|SetmembersinDS_UpgradeInfo NewParam))
  (Development|PrintString (Utilities|String|ToString(Float) (Utilities|Struct|BreakDS_UpgradeInfo _structout)) true true "(R=0.129585,G=1.000000,B=0.000000,A=1.000000)")
  (return _structout))

(fn TakeSkatesOff
  (Components|Capsule|SetCapsuleHalfHeight (Variables|/Script/Engine.Character|GetCapsuleComponent (CallFunction|GetPlayerCharacter)) 67.496719 true)
  (Rendering|SetVisibility (Variables|/Game/Player/BP_PlayerCharacter.BP_PlayerCharacter_C|GetRollerSkatesL (CallFunction|GetPlayerCharacter)) false false)
  (if (Variables|Default|GetHasBoostOn?)
    ;[0.15 0.15 0.15 0.5] If boost is on, the base speed == boosted speed
    (bind _output_get (Variables|Default|SetCurrentPlayerSpeed (Variables|Default|GetBoostedSpeed)))
    (bind _output_get_2 (Variables|/Script/Engine.CharacterMovementComponent|SetMaxWalkSpeed (Variables|/Script/Engine.Character|GetCharacterMovement (CallFunction|GetPlayerCharacter)) _output_get))
    (Development|PrintString (Utilities|String|Append "Set speed to: " (Utilities|String|ToString(Float) _output_get_2)) true true "(R=0.000000,G=1.000000,B=0.075772,A=1.000000)")
    (else
      ;[0.15 0.15 0.15 0.5] If no boos currently on, skates off will revert to base speed
      (bind _output_get_3 (Variables|Default|SetCurrentPlayerSpeed (Variables|Default|GetBaseSpeed)))
      (bind _output_get_4 (Variables|/Script/Engine.CharacterMovementComponent|SetMaxWalkSpeed (Variables|/Script/Engine.Character|GetCharacterMovement (CallFunction|GetPlayerCharacter)) _output_get_3))
      (Development|PrintString (Utilities|String|Append "Set speed to: " (Utilities|String|ToString(Float) _output_get_4)) true true "(R=0.000000,G=1.000000,B=0.075772,A=1.000000)"))))

(fn PuttingSkateson
  (bind _skatespeed (Variables|Default|GetSkateSpeed))
  (Rendering|SetVisibility (Variables|/Game/Player/BP_PlayerCharacter.BP_PlayerCharacter_C|GetRollerSkatesR (CallFunction|GetPlayerCharacter)) true false)
  (Components|Capsule|SetCapsuleHalfHeight (Variables|/Script/Engine.Character|GetCapsuleComponent (CallFunction|GetPlayerCharacter)) 7e+01 true)
  (bind _output_get (Variables|/Script/Engine.CharacterMovementComponent|SetMaxWalkSpeed (Variables|/Script/Engine.Character|GetCharacterMovement (CallFunction|GetPlayerCharacter)) (* (Variables|Default|GetCurrentPlayerSpeed) _skatespeed)))
  (bind _output_get_2 (Variables|Default|SetCurrentPlayerSpeed _output_get))
  (Development|PrintString "Skates on" true true "(R=1.000000,G=0.000000,B=0.633330,A=1.000000)")
  (Development|PrintString (Utilities|String|Append "Current multi: " (Utilities|String|ToString(Float) _skatespeed) " 
Current speed: " (Utilities|String|ToString(Float) _output_get_2)) true true "(R=0.555830,G=0.000000,B=1.000000,A=1.000000)"))