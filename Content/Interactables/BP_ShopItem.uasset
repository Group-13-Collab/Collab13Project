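; BP_ShopItem is a purchasable interactable that displays an upgrade's name and price.
; Its construction script uniformly scales the mesh from its Z bounds and MaxItemHeight, then fills the text labels.
; Looking at it broadcasts name, description and price.
; Interacting checks money in the player's quest log component, deducts the price, plays a register sound and returns Purchased, a stub returning false.
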(event EventItemLookedat
  (|CallParentFunction)
  (Default|CallOnLookedat (Variables|Default|GetItem%20Name) (Variables|Default|GetItem%20Description) (Variables|Default|GetItem%20Price)))

(fn ConstructionScript
  (bind _staticmesh (Variables|Default|GetStaticMesh))
  (bind _maxitemheight (Variables|Default|GetMaxItemHeight))
  (bind _staticmesh_2 (Variables|/Script/Engine.StaticMeshComponent|GetStaticMesh _staticmesh))
  (bind _returnvalue (StaticMesh|GetBounds _staticmesh_2))
  (bind _boxextent (Math|BoxSphereBounds|BreakBoxSphereBounds _returnvalue))
  (bind _z (Math|Vector|BreakVector _boxextent))
  (bind _returnvalue_2 (/ _maxitemheight _z))
  (|CallParentFunction)
  (Transformation|SetRelativeScale3D _staticmesh (Math|Vector|MakeVector _returnvalue_2 _returnvalue_2 _returnvalue_2))
  ;[0.15 0.15 0.15 0.5] ItemDesc
  (Rendering|Components|TextRender|SetText (Variables|Default|GetItemName) (Utilities|Struct|BreakDS_UpgradeInfo (Variables|Default|GetUpgradeData)))
  (Rendering|Components|TextRender|SetText (Variables|Default|GetPrice) (|GenerictoText (Utilities|String|Append "Item price: " (Utilities|String|ToString(Integer) (Variables|Default|GetItem%20Price))))))

(fn Interactedwith
  (bind _playercharacter (CallFunction|GetPlayerCharacter))
  (bind _item_price (Variables|Default|GetItem%20Price))
  (bind _bpc_questlog (Variables|/Game/Player/BP_PlayerCharacter.BP_PlayerCharacter_C|GetBPC_QuestLog _playercharacter))
  (if (>= (Variables|/Game/QuestSystem/BPC_QuestLog.BPC_QuestLog_C|GetMoney _bpc_questlog) _item_price)
    (Default|ChangeMoney _bpc_questlog (* _item_price -1))
    (Audio|PlaySound2D "/Game/Audio/SFX/Metasound/MS_Cash_Register.MS_Cash_Register" 1.0 1.0 0.0 0 0)
    (bind _isconsumedonpurchase (CallFunction|Purchased))
    (return _isconsumedonpurchase)
    (else
      (return false))))

(fn Purchased
  (return false))