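; BP_InteractableParent is the base actor for interactables that highlight when looked at and can be used through IA_Interact.
; Look events toggle custom depth on StaticMesh, with ColourMask set as its stencil value at BeginPlay, and enable or disable input so the actor only responds while looked at.
; On interact, it destroys itself if InteractedWith returns true.
; InteractedWith, InteractWith and GetReputation return only placeholder defaults here.
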(event Input|EnhancedActionEvents|EnhancedInputActionIA_Interact
  (params (ActionValue :type Boolean) (ElapsedSeconds :type Float%20%28double-precision%29) (TriggeredSeconds :type Float%20%28double-precision%29) (InputAction :type Input%20Action%20Object%20Reference :default "/Game/Inputs/PlayerInputs/IA_Interact.IA_Interact"))
  (:Started
    (bind _isdestroyed (CallFunction|Interactedwith))
    (if _isdestroyed
      (Actor|DestroyActor))))

(event EventBeginPlay
  (Rendering|SetCustomDepthStencilValue (Variables|Default|GetStaticMesh) (Variables|Default|GetColourMask)))

(event EventItemStopLookedat
  (Rendering|SetRenderCustomDepth (Variables|Default|GetStaticMesh) false)
  (Input|DisableInput (Game|GetPlayerController 0)))

(event EventItemLookedat
  (Rendering|SetRenderCustomDepth (Variables|Default|GetStaticMesh) true)
  (Input|EnableInput (Game|GetPlayerController 0)))

(fn ConstructionScript)

(fn Interactedwith
  (return false))

(fn GetReputation
  (return "NewEnumerator0"))

(fn Interactwith
  (params (IsQuestCompleted? :type Boolean) (ReputationType :type E_Reputation%20Enum :default "NewEnumerator0"))
  (return ""))