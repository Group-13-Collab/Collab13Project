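; Quest-giver NPC that patrols a spline, handles dialogue and tracks its reputation in three tiers.
; Tick moves only the mesh along the spline with fixed offsets, sets a constant movement velocity, and optionally loops.
; InteractWith forwards to the dialogue component and leaves InteractedWith true, halting the patrol.
; Reputation gains are scaled by the player's Rep upgrade, then the tier is recalculated by thresholds.
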(event EventBeginPlay)

(event EventTick
  (params (DeltaSeconds :type Float%20%28single-precision%29))
  (bind _mesh (Variables|Character|GetMesh))
  (if (not (Variables|Default|GetInteractedWith?))
    (Variables|Default|SetDistanceAlongSpline (+ (* DeltaSeconds (Variables|Default|GetSpline%20Speed)) (Variables|Default|GetDistanceAlongSpline)))
    (Transformation|SetRelativeTransform _mesh (Math|Transform|MakeTransform (Math|Vector|MakeVector (.x (.location (Spline|GetTransformatDistanceAlongSpline (Variables|Default|GetSpline) (Variables|Default|GetDistanceAlongSpline) "Local" false))) (.y (.location (Spline|GetTransformatDistanceAlongSpline (Variables|Default|GetSpline) (Variables|Default|GetDistanceAlongSpline) "Local" false))) (+ (.z (.location (Spline|GetTransformatDistanceAlongSpline (Variables|Default|GetSpline) (Variables|Default|GetDistanceAlongSpline) "Local" false))) -89.0)) (Math|Rotator|MakeRotator (.roll (.rotation (Spline|GetTransformatDistanceAlongSpline (Variables|Default|GetSpline) (Variables|Default|GetDistanceAlongSpline) "Local" false))) (.pitch (.rotation (Spline|GetTransformatDistanceAlongSpline (Variables|Default|GetSpline) (Variables|Default|GetDistanceAlongSpline) "Local" false))) (+ (.yaw (.rotation (Spline|GetTransformatDistanceAlongSpline (Variables|Default|GetSpline) (Variables|Default|GetDistanceAlongSpline) "Local" false))) -9e+01)) (Variables|/Script/Engine.SceneComponent|GetRelativeScale3D _mesh)) false false)
    (Variables|/Script/Engine.MovementComponent|SetVelocity (Variables|Character|GetCharacterMovement) "120.000000,0.000000,0.000000")
    (if (Variables|Default|Getloop)
      (if (> (Variables|Default|GetDistanceAlongSpline) (Spline|GetSplineLength (Variables|Default|GetSpline)))
        (Variables|Default|SetDistanceAlongSpline 0.0)))))

(event EventUpdateReputationPoints
  (params (Points :type Float%20%28double-precision%29))
  (bind _bpc_reputation (Variables|Default|GetBPC_Reputation))
  (bind _output_get (Variables|/Game/Reputation/BPC_Reputation.BPC_Reputation_C|SetReputationValue _bpc_reputation (+ (* Points (Utilities|Struct|BreakDS_UpgradeInfo (Variables|/Game/Interactables/Upgrades/BPC_Upgrades.BPC_Upgrades_C|GetUpgradeInfo (Variables|/Game/Player/BP_PlayerCharacter.BP_PlayerCharacter_C|GetBPC_Upgrades (CallFunction|GetPlayerCharacter))))) (Variables|/Game/Reputation/BPC_Reputation.BPC_Reputation_C|GetReputationValue _bpc_reputation))))
  (CallFunction|UpdateReputationType)
  (Development|PrintString (Utilities|String|ToString(Float) _output_get)))

(fn ConstructionScript)

(fn UpdateReputationType
  (bind _bpc_reputation (Variables|Default|GetBPC_Reputation))
  (bind _bpc_reputation_2 (Variables|Default|GetBPC_Reputation))
  (bind _reputationvalue (Variables|/Game/Reputation/BPC_Reputation.BPC_Reputation_C|GetReputationValue _bpc_reputation_2))
  (if (> _reputationvalue 5e+01)
    (bind _output_get (Variables|/Game/Reputation/BPC_Reputation.BPC_Reputation_C|SetReputationType _bpc_reputation_2 "NewEnumerator0"))
    (Variables|/Game/Reputation/BPC_Reputation.BPC_Reputation_C|SetReputationType _bpc_reputation _output_get)
    (elif (< _reputationvalue 1e+01)
      (bind _output_get_2 (Variables|/Game/Reputation/BPC_Reputation.BPC_Reputation_C|SetReputationType _bpc_reputation_2 "NewEnumerator2"))
      (Variables|/Game/Reputation/BPC_Reputation.BPC_Reputation_C|SetReputationType _bpc_reputation _output_get_2)
      (else
        (bind _output_get_3 (Variables|/Game/Reputation/BPC_Reputation.BPC_Reputation_C|SetReputationType _bpc_reputation_2 "NewEnumerator1"))
        (Variables|/Game/Reputation/BPC_Reputation.BPC_Reputation_C|SetReputationType _bpc_reputation _output_get_3)))))

(fn GetReputation
  (return (Variables|/Game/Reputation/BPC_Reputation.BPC_Reputation_C|GetReputationType (Variables|Default|GetBPC_Reputation))))

(fn Interactwith
  (params (IsQuestCompleted? :type Boolean) (ReputationType :type E_Reputation%20Enum :default "NewEnumerator0"))
  (Variables|Default|SetInteractedWith? false)
  (bind _objectiveid (Default|Interactwith (Variables|Default|GetBPC_DialogueTest) IsQuestCompleted? ReputationType))
  (Variables|Default|SetInteractedWith? true)
  (return _objectiveid))