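; BP_Ocean is an ocean ambience actor that keeps its sound on the point of a shoreline-style spline nearest the player.
; On BeginPlay it caches the player character and starts a self-calling MoveAudio event with a 0.1-second delay.
; Each pass moves the Audio component to the closest spline point to the player, raised slightly in Z, so the sound follows along the spline.
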(event Custom|Move%20Audio
  (bind _player_character (Variables|Default|GetPlayer%20Character))
  (bind _spline (Variables|Default|GetSpline))
  (bind _returnvalue (Transformation|GetActorLocation _player_character))
  (bind _returnvalue_2 (Spline|FindLocationClosesttoWorldLocation _spline _returnvalue "World"))
  (Transformation|SetWorldLocation (Variables|Default|GetAudio) (Math|Vector|MakeVector (.x _returnvalue_2) (.y _returnvalue_2) (+ (.z _returnvalue_2) 5e+01)) false false)
  (Utilities|FlowControl|Delay 0.1)
  (CallFunction|MoveAudio))

(event EventBeginPlay
  (Variables|Default|SetPlayer%20Character (CallFunction|GetPlayerCharacter))
  (CallFunction|MoveAudio))

(fn ConstructionScript)