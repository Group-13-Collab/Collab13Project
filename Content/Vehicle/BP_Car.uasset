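; Drivable car pawn built on Chaos wheeled vehicle movement, with an exit back to the on-foot player character.
; Enhanced Input actions drive camera look, steering, and a single forward/backward axis that feeds throttle and, negated, brake, with inputs zeroed on release.
; Interact finds BP_PlayerCharacter by class, teleports it to the PlayerVehicleExit transform, unhides it and has player controller 0 possess it.
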(event Input|EnhancedActionEvents|EnhancedInputActionIA_VehicleForwardBackward
  (params (ActionValue :type Float%20%28double-precision%29) (ElapsedSeconds :type Float%20%28double-precision%29) (TriggeredSeconds :type Float%20%28double-precision%29) (InputAction :type Input%20Action%20Object%20Reference :default "/Game/Inputs/VehicleInputs/IA_VehicleForwardBackward.IA_VehicleForwardBackward"))
  (bind _chaoswheeledvehiclemovement (Variables|Default|GetChaosWheeledVehicleMovement))
  (bind _chaoswheeledvehiclemovement_2 (Variables|Default|GetChaosWheeledVehicleMovement))
  (:Triggered
    (Class|ChaosVehicleMovementComponent|SetThrottleInput _chaoswheeledvehiclemovement_2 ActionValue)
    (Class|ChaosVehicleMovementComponent|SetBrakeInput _chaoswheeledvehiclemovement_2 (* ActionValue -1.0)))
  (:Completed
    (Class|ChaosVehicleMovementComponent|SetThrottleInput _chaoswheeledvehiclemovement 0.0)
    (Class|ChaosVehicleMovementComponent|SetBrakeInput _chaoswheeledvehiclemovement (* 0.0 -1.0))))

(event Input|EnhancedActionEvents|EnhancedInputActionIA_VehicleLeftRight
  (params (ActionValue :type Float%20%28double-precision%29) (ElapsedSeconds :type Float%20%28double-precision%29) (TriggeredSeconds :type Float%20%28double-precision%29) (InputAction :type Input%20Action%20Object%20Reference :default "/Game/Inputs/VehicleInputs/IA_VehicleLeftRight.IA_VehicleLeftRight"))
  (:Triggered
    (Class|ChaosVehicleMovementComponent|SetSteeringInput (Variables|Default|GetChaosWheeledVehicleMovement) ActionValue))
  (:Completed
    (Class|ChaosVehicleMovementComponent|SetSteeringInput (Variables|Default|GetChaosWheeledVehicleMovement) 0.0)))

(event Input|EnhancedActionEvents|EnhancedInputActionIA_Look
  (params (ActionValue :type Vector%202D%20Structure) (ElapsedSeconds :type Float%20%28double-precision%29) (TriggeredSeconds :type Float%20%28double-precision%29) (InputAction :type Input%20Action%20Object%20Reference :default "/Game/Inputs/PlayerInputs/IA_Look.IA_Look"))
  (bind (_x _y) (Math|Vector2D|BreakVector2D ActionValue))
  (Pawn|Input|AddControllerYawInput _x)
  (Pawn|Input|AddControllerPitchInput _y))

(event Input|EnhancedActionEvents|EnhancedInputActionIA_Interact
  (params (ActionValue :type Boolean) (ElapsedSeconds :type Float%20%28double-precision%29) (TriggeredSeconds :type Float%20%28double-precision%29) (InputAction :type Input%20Action%20Object%20Reference :default "/Game/Inputs/PlayerInputs/IA_Interact.IA_Interact"))
  (bind _playervehicleexit (Variables|Default|GetPlayerVehicleExit))
  (bind _returnvalue (Transformation|GetWorldTransform _playervehicleexit))
  (bind _returnvalue_2 (Actor|GetActorOfClass "/Game/Player/BP_PlayerCharacter.BP_PlayerCharacter_C"))
  (Transformation|SetActorTransform _returnvalue_2 (Math|Transform|MakeTransform (.location _returnvalue) (.rotation _returnvalue) "1.000000,1.000000,1.000000") false true)
  (Rendering|SetActorHiddenInGame _returnvalue_2 false)
  (Pawn|Possess (Game|GetPlayerController 0) _returnvalue_2))

(fn ConstructionScript)