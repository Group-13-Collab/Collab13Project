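; A bird actor that repeatedly flies along a referenced spline as environmental dressing.
; On BeginPlay, a timeline with play rate scaled by TimeToComplete maps its track to distance along the spline, setting world location and rotation each update.
; When the timeline finishes, it waits a fixed delay and restarts from the spline's beginning.
; The construction script sets the bird's skeletal mesh asset.
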(event Custom|Move%20Object
  (bind _spline_to_follow (Variables|Default|GetSpline%20To%20Follow))
  (bind _spline (Variables|/Game/Environment/Misc/Birds/BP_BirdSpline.BP_BirdSpline_C|GetSpline _spline_to_follow))
  (Components|Timeline|SetPlayRate (Variables|Default|GetT_Move) (/ 1.0 (Variables|Default|GetTime%20To%20Complete)))
  (bind _move_track (Timeline|T_Move PlayFromStart)
    (:Update
      (Transformation|SetActorLocationAndRotation (Spline|GetLocationatDistanceAlongSpline _spline (Math|Float|Lerp 0.0 (Spline|GetSplineLength _spline) _move_track) "World") (Spline|GetRotationatDistanceAlongSpline _spline (Math|Float|Lerp 0.0 (Spline|GetSplineLength _spline) _move_track) "World")))
    (:Finished
      (Utilities|FlowControl|Delay 1e+01)
      (CallFunction|MoveObject))))

(event EventBeginPlay
  (CallFunction|MoveObject))

(fn ConstructionScript
  (Components|SkeletalMesh|SetSkeletalMeshAsset (Variables|Default|GetBIRDANIMATIONRAHHHH) "/Game/Environment/Misc/Birds/Models/BIRDANIMATIONRAHHHH.BIRDANIMATIONRAHHHH"))