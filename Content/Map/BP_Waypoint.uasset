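; BP_Waypoint is a world waypoint actor that shows the player's distance to it on a widget component.
; On BeginPlay it casts the widget to WBP_Waypoint and caches its TXTDistance text element.
; Every Tick it measures the distance to player pawn 0, converts it to whole meters and writes it to that text with an "m" suffix.
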(event EventBeginPlay
  (bind _aswbp_waypoint (Utilities|Casting|CastToWBP_Waypoint (UserInterface|GetWidget (Variables|Default|GetWidget))))
  (Variables|Default|SetTXT%20Distance (Variables|/Game/UI/WBP_Waypoint.WBP_Waypoint_C|GetTXT_Distance _aswbp_waypoint)))

(event EventTick
  (params (DeltaSeconds :type Float%20%28single-precision%29))
  (Rendering|Components|TextRender|SetText (Variables|Default|GetTXT%20Distance) (Utilities|Text|ToText(String) (Utilities|String|Append (Utilities|String|ToString(Integer) (Math|Float|Truncate (/ (Math|Vector|Distance(Vector) (Transformation|GetActorLocation) (Transformation|GetActorLocation (Game|Player|GetPlayerPawn 0))) 1e+02))) " m"))))

(fn ConstructionScript)