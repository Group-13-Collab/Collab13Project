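; Quest log component that tracks active and completed quests along with the player's money.
; Adding a quest spawns a BP_QuestBase actor, found later by ID, and calls Marker on matching BP_LocationMarker actors.
; Turn-in pays the stage reward scaled by upgrade and reputation multipliers, then completes the quest, updating the game mode counter, player message and markers.
; ChangeMoney broadcasts balance changes, while turn-in edits Money directly; TrackQuest is empty.
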(fn AddNewQuest
  (params (QuestID :type Name))
  ;[0.15 0.15 0.15 0.5] Adds widget to the quest log and to the current quest array
  (Utilities|Array|AddUnique (Variables|Default|GetCurrentActiveQuests) QuestID)
  (bind _returnvalue (Game|SpawnActorfromClass "/Game/QuestSystem/BP_QuestBase.BP_QuestBase_C" (Math|Transform|MakeTransform "0, 0, 0" "0, 0, 0" "1.000000,1.000000,1.000000") "Undefined" "MultiplyWithRoot" 0 QuestID false 0))
  (Utilities|Array|Add (Variables|Default|GetCurrentQuests) _returnvalue)
  (bind _outactors (Actor|GetAllActorsOfClass "/Game/QuestSystem/BP_LocationMarker.BP_LocationMarker_C"))
  (for _array_element _outactors
    (if (Utilities|Enum|Equal(Enum) (Variables|/Game/QuestSystem/BP_LocationMarker.BP_LocationMarker_C|GetObjectiveID _array_element) (Utilities|String|ToString(Name) QuestID))
      (Default|Marker _array_element (Variables|/Game/QuestSystem/BP_LocationMarker.BP_LocationMarker_C|GetObjectiveID _array_element))))
  (return _returnvalue))

(fn CompleteQuest
  (params (QuestID :type Name%20%28by%20ref%29))
  (bind _gamemode (Variables|Default|GetGamemode))
  ;[0.15 0.15 0.15 0.5] Adds quest to the completed quest while removing from active quests, after checks the quest as turned in.
  (Utilities|Array|AddUnique (Variables|Default|GetCompletedQuests) QuestID)
  (Utilities|Array|RemoveItem (Variables|Default|GetCurrentActiveQuests) QuestID)
  (bind _array_element (CallFunction|GetQuestActor QuestID))
  (Default|CallOnQuestCompleted _array_element)
  (bind _output_get (Variables|/Game/QuestSystem/BP_QuestBase.BP_QuestBase_C|SetIsTurnedIn _array_element true))
  (Variables|Default|SetIsQuestCompleted? true)
  (Variables|/Game/BP_MainGamemode.BP_MainGamemode_C|SetQuestCounter _gamemode (+ (Variables|/Game/BP_MainGamemode.BP_MainGamemode_C|GetQuestCounter _gamemode) 1))
  (Class|BPIPlayerInformation|SetIsQuestCompleted(Message) (Game|GetPlayerCharacter 0) _output_get 0.0 0.0)
  (bind _outactors (Actor|GetAllActorsOfClass "/Game/QuestSystem/BP_LocationMarker.BP_LocationMarker_C"))
  (for _array_element_2 _outactors
    (if (Utilities|Enum|Equal(Enum) (Variables|/Game/QuestSystem/BP_LocationMarker.BP_LocationMarker_C|GetObjectiveID _array_element_2) (Utilities|String|ToString(Name) QuestID))
      (Default|Marker _array_element_2 (Variables|/Game/QuestSystem/BP_LocationMarker.BP_LocationMarker_C|GetObjectiveID _array_element_2)))))

(fn ActiveQuestQuery
  (params (QuestID :type Name))
  ;[0.15 0.15 0.15 0.5] Check if quest id is in active quests
  (return (Utilities|Array|ContainsItem (Variables|Default|GetCurrentActiveQuests) QuestID)))

(fn TrackQuest)

(fn GetQuestActor
  (params (QuestID :type Name))
  ;[0.15 0.15 0.15 0.5] Loops through current quests and checks quest id to the ones stored in the array and if they are the same it will return
  (for _array_element (Variables|Default|GetCurrentQuests)
    (if (== (Variables|/Game/QuestSystem/BP_QuestBase.BP_QuestBase_C|GetQuestID _array_element) QuestID)
      (return _array_element))))

(fn TurninQuest
  (params (QuestID :type Name))
  ;[0.15 0.15 0.15 0.5] Turns in quest, gives rewards and marks it as complete
  (Utilities|FlowControl|Sequence
    (:then_0
      (bind _array_element (CallFunction|GetQuestActor QuestID))
      (bind _structout (Utilities|Struct|SetmembersinDS_UpgradeInfo (Variables|/Game/Interactables/Upgrades/BPC_Upgrades.BPC_Upgrades_C|GetUpgradeInfo (Variables|/Game/Player/BP_PlayerCharacter.BP_PlayerCharacter_C|GetBPC_Upgrades (CallFunction|GetPlayerCharacter)))))
      (switch Utilities|FlowControl|Switch|SwitchonE_Reputation (Variables|Default|GetCurrentReputation)
        (:NewEnumerator0
          (Variables|Default|SetMoney (+ (Variables|Default|GetMoney) (Math|Float|Truncate (* (* (.MoneyReward (Utilities|Struct|BreakF_StageDetails (Variables|/Game/QuestSystem/BP_QuestBase.BP_QuestBase_C|GetCurrentStageDetails _array_element))) (Utilities|Struct|BreakDS_UpgradeInfo _structout)) (Variables|Default|GetHappyMult))))))
        (:NewEnumerator1
          (Variables|Default|SetMoney (+ (Variables|Default|GetMoney) (Math|Float|Truncate (* (* (.MoneyReward (Utilities|Struct|BreakF_StageDetails (Variables|/Game/QuestSystem/BP_QuestBase.BP_QuestBase_C|GetCurrentStageDetails _array_element))) (Utilities|Struct|BreakDS_UpgradeInfo _structout)) (Variables|Default|GetNeutralMult))))))
        (:NewEnumerator2
          (Variables|Default|SetMoney (+ (Math|Float|Truncate (* (* (.MoneyReward (Utilities|Struct|BreakF_StageDetails (Variables|/Game/QuestSystem/BP_QuestBase.BP_QuestBase_C|GetCurrentStageDetails _array_element))) (Utilities|Struct|BreakDS_UpgradeInfo _structout)) (Variables|Default|GetUnhappyMult))) (Variables|Default|GetMoney)))))
      (Audio|PlaySound2D "/Game/Audio/SFX/Metasound/MS_Coins.MS_Coins" 1.0 1.0 0.0 0 0))
    (:then_1
      (CallFunction|CompleteQuest QuestID))))

(fn CompleteQuestQuery
  (params (QuestID :type Name))
  (bind _completedquests (Variables|Default|GetCompletedQuests))
  (bind _returnvalue (Utilities|Array|ContainsItem _completedquests QuestID))
  ;[0.15 0.15 0.15 0.5] Adds quest to completed quest array and marks it as complete
  (bind _array_element (CallFunction|GetQuestActor QuestID))
  (Utilities|IsValid _array_element
    (:Is%20Valid
      (return _returnvalue (Variables|/Game/QuestSystem/BP_QuestBase.BP_QuestBase_C|GetIsTurnedIn _array_element)))
    (:Is%20Not%20Valid
      (return _returnvalue false))))

(fn ChangeMoney
  (params (Change :type Integer))
  ;[0.15 0.15 0.15 0.5] Changes amount of money
  (bind _output_get (Variables|Default|SetMoney (+ (Variables|Default|GetMoney) Change)))
  (Default|CallOnMoneyChanged _output_get)
  (return))