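; Quest giver actor component that offers one of two data table quests and shows reward widgets, choosing the second once the player's quest log lists the first as completed.
; DisplayQuest and DisplayRewards build the widgets from quest rows; the latter also sets MoneyReward per stage, adjusted by the owner's BPC_Reputation mood.
; InteractWith is empty, with its quest-state branching left disconnected, and GetReputation always returns Happy.
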(fn DisplayQuest
  (bind _firstquest (Variables|Default|GetFirstQuest))
  (bind _secondquest (Variables|Default|GetSecondQuest))
  ;[0.15 0.15 0.15 0.5] Displays the Give Quest Widget
  (if (Utilities|Array|ContainsItem (Variables|/Game/QuestSystem/BPC_QuestLog.BPC_QuestLog_C|GetCompletedQuests (Variables|/Game/Player/BP_PlayerCharacter.BP_PlayerCharacter_C|GetBPC_QuestLog (CallFunction|GetPlayerCharacter))) (.rowname _firstquest))
    (bind _returnvalue (Utilities|GetDataTableRow (.datatable _secondquest) (.rowname _secondquest))
      (:then
        (bind _returnvalue_2 (UserInterface|CreateWidget "/Game/QuestSystem/UI/WBP_QuestGiver.WBP_QuestGiver_C" 0 _returnvalue (.rowname _secondquest)))
        (UserInterface|Viewport|AddtoViewport _returnvalue_2 0)))
    (else
      (bind _returnvalue_3 (Utilities|GetDataTableRow (.datatable _firstquest) (.rowname _firstquest))
        (:then
          (bind _returnvalue_4 (UserInterface|CreateWidget "/Game/QuestSystem/UI/WBP_QuestGiver.WBP_QuestGiver_C" 0 _returnvalue_3 (.rowname _firstquest)))
          (UserInterface|Viewport|AddtoViewport _returnvalue_4 0))))))

(fn DisplayRewards
  (bind _firstquest (Variables|Default|GetFirstQuest))
  (bind _secondquest (Variables|Default|GetSecondQuest))
  ;[0.15 0.15 0.15 0.5] Display Quest Rewards
  (if (Utilities|Array|ContainsItem (Variables|/Game/QuestSystem/BPC_QuestLog.BPC_QuestLog_C|GetCompletedQuests (Variables|/Game/Player/BP_PlayerCharacter.BP_PlayerCharacter_C|GetBPC_QuestLog (CallFunction|GetPlayerCharacter))) (.rowname (Variables|Default|GetFirstQuest)))
    ;[0.15 0.15 0.15 0.5] Second Quest Rewards
    (bind _returnvalue (Utilities|GetDataTableRow (.datatable _secondquest) (.rowname _secondquest))
      (:then
        (bind _returnvalue_2 (UserInterface|CreateWidget "/Game/QuestSystem/UI/WBP_QuestRewards.WBP_QuestRewards_C" 0 _returnvalue (.rowname _secondquest)))
        (UserInterface|Viewport|AddtoViewport _returnvalue_2 0)
        (bind _array_element (Utilities|Array|ForEachLoopwithBreak (.Stages (Utilities|Struct|BreakF_QuestDetails _returnvalue)))
          (:LoopBody
            (switch Utilities|FlowControl|Switch|SwitchonE_Reputation (Variables|/Game/Reputation/BPC_Reputation.BPC_Reputation_C|GetReputationType (Actor|GetComponentbyClass (Components|GetOwner) "/Game/Reputation/BPC_Reputation.BPC_Reputation_C"))
              (:NewEnumerator0
                (Variables|Default|SetMoneyReward (+ (* (.MoneyReward (Utilities|Struct|BreakF_StageDetails _array_element)) 0.2) (.MoneyReward (Utilities|Struct|BreakF_StageDetails _array_element)))))
              (:NewEnumerator1
                (Variables|Default|SetMoneyReward (Math|Conversions|ToFloat(Integer) (.MoneyReward (Utilities|Struct|BreakF_StageDetails _array_element)))))
              (:NewEnumerator2
                (Variables|Default|SetMoneyReward (- (.MoneyReward (Utilities|Struct|BreakF_StageDetails _array_element)) (* (.MoneyReward (Utilities|Struct|BreakF_StageDetails _array_element)) 0.2)))))))))
    (else
      ;[0.15 0.15 0.15 0.5] First Quest Rewards
      (bind _returnvalue_3 (Utilities|GetDataTableRow "/Game/QuestSystem/QuestData/QuestData.QuestData" (.rowname _firstquest))
        (:then
          (bind _returnvalue_4 (UserInterface|CreateWidget "/Game/QuestSystem/UI/WBP_QuestRewards.WBP_QuestRewards_C" 0 _returnvalue_3 (.rowname _firstquest)))
          (UserInterface|Viewport|AddtoViewport _returnvalue_4 0)
          (bind _array_element_2 (Utilities|Array|ForEachLoopwithBreak (.Stages (Utilities|Struct|BreakF_QuestDetails _returnvalue_3)))
            (:LoopBody
              (switch Utilities|FlowControl|Switch|SwitchonE_Reputation (Variables|/Game/Reputation/BPC_Reputation.BPC_Reputation_C|GetReputationType (Actor|GetComponentbyClass (Components|GetOwner) "/Game/Reputation/BPC_Reputation.BPC_Reputation_C"))
                (:NewEnumerator0
                  (Variables|Default|SetMoneyReward (+ (* (.MoneyReward (Utilities|Struct|BreakF_StageDetails _array_element_2)) 0.2) (.MoneyReward (Utilities|Struct|BreakF_StageDetails _array_element_2)))))
                (:NewEnumerator1
                  (Variables|Default|SetMoneyReward (Math|Conversions|ToFloat(Integer) (.MoneyReward (Utilities|Struct|BreakF_StageDetails _array_element_2)))))
                (:NewEnumerator2
                  (Variables|Default|SetMoneyReward (- (.MoneyReward (Utilities|Struct|BreakF_StageDetails _array_element_2)) (* (.MoneyReward (Utilities|Struct|BreakF_StageDetails _array_element_2)) 0.2))))))))))))

(fn GetReputation
  (return "NewEnumerator0"))

(fn Interactwith
  (params (IsQuestCompleted? :type Boolean) (ReputationType :type E_Reputation%20Enum :default "NewEnumerator0")))