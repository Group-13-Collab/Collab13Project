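; BP_LocationMarker is a quest waypoint that shows the player's distance in meters through a waypoint widget, updated every tick.
; Marker and MarkerOff toggle that widget for a matching ObjectiveID.
; Player overlap reports the objective ID to the player character, shows a location notification, then destroys the marker.
; The "endlocation" marker, when all quests are complete, instead fades to black and opens the main menu.
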(event Custom|MarkerOff
  (params (LoopObjectiveID :type String))
  (if (Utilities|Enum|Equal(Enum) LoopObjectiveID (Variables|Default|GetObjectiveID))
    (Rendering|SetVisibility (Variables|Default|GetWidget) false false)))

(event Custom|Marker
  (params (LoopObjectiveID :type String))
  (if (Utilities|Enum|Equal(Enum) LoopObjectiveID (Variables|Default|GetObjectiveID))
    (Rendering|SetVisibility (Variables|Default|GetWidget) true false)))

(event EventBeginPlay
  (bind _aswbp_waypoint (Utilities|Casting|CastToWBP_Waypoint (UserInterface|GetWidget (Variables|Default|GetWidget))))
  (Variables|Default|SetTXT%20Distance (Variables|/Game/UI/WBP_Waypoint.WBP_Waypoint_C|GetTXT_Distance _aswbp_waypoint)))

(event Collision|EventActorBeginOverlap
  (params (OtherActor :type Actor%20Object%20Reference))
  ;[0.15 0.15 0.15 0.5] Lets Quest Base know that a task has been complete
  (bind _asbp_player_character (Utilities|Casting|CastToBP_PlayerCharacter OtherActor))
  (Default|CallOnObjectiveIDCalled _asbp_player_character (Variables|Default|GetObjectiveID))
  (bind _returnvalue (UserInterface|CreateWidget "/Game/QuestSystem/UI/WBP_LocationNotify.WBP_LocationNotify_C" 0 (Variables|Default|GetLocationName)))
  (UserInterface|Viewport|AddtoViewport _returnvalue 0)
  (if (and (Utilities|Enum|Equal(Enum) (Variables|Default|GetObjectiveID) "endlocation") (Variables|/Game/BP_MainGamemode.BP_MainGamemode_C|GetAllQuestsComplete (Variables|Default|GetGamemode)))
    (bind _returnvalue_2 (UserInterface|CreateWidget "/Game/UI/WBP_FadeToBlack.WBP_FadeToBlack_C"))
    (Default|FadetoBlack _returnvalue_2)
    (Utilities|FlowControl|Delay 2.0)
    (Game|OpenLevel(byName) "MainMenu")
    (else
      (Actor|DestroyActor))))

(event EventTick
  (params (DeltaSeconds :type Float%20%28single-precision%29))
  (Rendering|Components|TextRender|SetText (Variables|Default|GetTXT%20Distance) (Utilities|Text|ToText(String) (Utilities|String|Append (Utilities|String|ToString(Integer) (Math|Float|Truncate (/ (Math|Vector|Distance(Vector) (Transformation|GetActorLocation) (Transformation|GetActorLocation (Game|Player|GetPlayerPawn 0))) 1e+02))) " m"))))

(fn ConstructionScript)