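; Save data object that persists quest log state, player money and audio volume settings.
; Separate save functions copy active and completed quests, money and volume levels, and record each quest's stage and objective progress in a map keyed by quest ID.
; LoadQuests re-adds active quests through the quest log component, restores their saved progress, then writes back the quest lists and money.
; LoadSound returns the stored volume levels.
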(fn SaveQuestDetails
  (params (Quest :type BP%20Quest%20Base%20Object%20Reference))
  (Utilities|Map|Add (Variables|Default|GetQuestProgress) (Variables|/Game/QuestSystem/BP_QuestBase.BP_QuestBase_C|GetQuestID Quest) (Utilities|Struct|MakeF_QuestSaveData (Variables|/Game/QuestSystem/BP_QuestBase.BP_QuestBase_C|GetCurrentObjectiveProgress Quest) (Variables|/Game/QuestSystem/BP_QuestBase.BP_QuestBase_C|GetCurrentStage Quest))))

(fn LoadQuests
  (params (QuestLogComponent :type BPC%20Quest%20Log%20Object%20Reference))
  ;[0.15 0.15 0.15 0.5] Gets the quests that have been saved, loops through them all adding them back to the quest log UI. Also adding back the amount of money that you had beforehand.
  (for _array_element (Variables|Default|GetCurrentActiveQuests)
    (bind _returnvalue (Default|AddNewQuest QuestLogComponent _array_element))
    (Variables|/Game/QuestSystem/BP_QuestBase.BP_QuestBase_C|SetCurrentStage _returnvalue (.CurrentStage (Utilities|Struct|BreakF_QuestSaveData (.Value (Utilities|Map|Find (Variables|Default|GetQuestProgress) _array_element)))))
    (Variables|/Game/QuestSystem/BP_QuestBase.BP_QuestBase_C|SetCurrentObjectiveProgress _returnvalue (.Progress (Utilities|Struct|BreakF_QuestSaveData (.Value (Utilities|Map|Find (Variables|Default|GetQuestProgress) _array_element))))))
  (Variables|/Game/QuestSystem/BPC_QuestLog.BPC_QuestLog_C|SetCurrentActiveQuests QuestLogComponent (Variables|Default|GetCurrentActiveQuests))
  (Variables|/Game/QuestSystem/BPC_QuestLog.BPC_QuestLog_C|SetCompletedQuests QuestLogComponent (Variables|Default|GetCompletedQuests))
  (Variables|/Game/QuestSystem/BPC_QuestLog.BPC_QuestLog_C|SetMoney QuestLogComponent (Variables|Default|GetMoney)))

(fn SaveQuestLog
  (params (QuestLog :type BPC%20Quest%20Log%20Object%20Reference))
  (Variables|Default|SetCurrentActiveQuests (Variables|/Game/QuestSystem/BPC_QuestLog.BPC_QuestLog_C|GetCurrentActiveQuests QuestLog))
  (Variables|Default|SetCompletedQuests (Variables|/Game/QuestSystem/BPC_QuestLog.BPC_QuestLog_C|GetCompletedQuests QuestLog)))

(fn SaveMoney
  (params (Quest%20Log :type BPC%20Quest%20Log%20Object%20Reference))
  (Variables|Default|SetMoney (Variables|/Game/QuestSystem/BPC_QuestLog.BPC_QuestLog_C|GetMoney Quest%20Log)))

(fn SaveVolume
  (params (Master%20Volume :type Float%20%28double-precision%29) (Music%20Volume :type Float%20%28double-precision%29) (UI%20Volume :type Float%20%28double-precision%29) (SFX%20Volume :type Float%20%28double-precision%29) (Environment%20Volume :type Float%20%28double-precision%29))
  (Variables|Default|SetVolumeStates (Utilities|Struct|MakeVolumeSaveStruct Master%20Volume Music%20Volume UI%20Volume SFX%20Volume Environment%20Volume)))

(fn LoadSound
  (bind _volumestates (Variables|Default|GetVolumeStates))
  (return (.mastervolume _volumestates) (.musicvolume _volumestates) (.uivolume _volumestates) (.sfxvolume _volumestates) (.environmentvolume _volumestates)))