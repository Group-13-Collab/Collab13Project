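; Base quest Blueprint that tracks one quest's staged objectives and detects when it is completed.
; It loads the current stage from the QuestData table by QuestID into a progress map keyed by objective ID.
; The player's OnObjectiveIDCalled dispatcher drives the counts, and each finished objective shows a notification widget.
; A finished stage loads the next; the last stops the GameMode's quest timer and reports completion and times to the player.
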(event EventBeginPlay
  (CallFunction|GetQuestDetails)
  (EventDispatchers|BindEventtoOnObjectiveIDCalled (CallFunction|GetPlayerCharacter) (EventDispatchers|CreateEvent :!event OnObjectiveIDHeard))
  (Utilities|FlowControl|Delay 0.2)
  (bind _return (CallFunction|IsAllObjectivesComplete))
  (Variables|Default|SetIsCompleted _return))

(fn ConstructionScript)

(fn OnObjectiveIDHeard
  (params (ObjectiveID :type String))
  (bind _currentobjectiveprogress (Variables|Default|GetCurrentObjectiveProgress))
  (bind (_value _returnvalue) (Utilities|Map|Find _currentobjectiveprogress ObjectiveID))
  (if _returnvalue
    (if (< _value (Utilities|Struct|BreakF_ObjectiveDetails (CallFunction|GetObjectiveDatabyID ObjectiveID)))
      (Utilities|Map|Add (Variables|Default|GetCurrentObjectiveProgress) ObjectiveID (+ _value 1))
      (CallFunction|IsObjectiveComplete ObjectiveID)
      (return))
    (else
      (return))))

(fn GetQuestDetails
  (bind _returnvalue (Utilities|GetDataTableRow "/Game/QuestSystem/QuestData/QuestData.QuestData" (Variables|Default|GetQuestID))
    (:then
      (bind _output_get (Variables|Default|SetQuestDetails _returnvalue))
      (bind _output_get_2 (Variables|Default|SetCurrentStageDetails (Utilities|Array|Get(acopy) (.Stages (Utilities|Struct|BreakF_QuestDetails _output_get)) (Variables|Default|GetCurrentStage))))
      (Utilities|Map|Clear (Variables|Default|GetCurrentObjectiveProgress))
      (Variables|Default|SetCompletion%20Time (.CompletionTime (Utilities|Struct|BreakF_StageDetails _output_get_2)))
      (for _array_element (.Objectives (Utilities|Struct|BreakF_StageDetails _output_get_2))
        (Development|PrintString (.ObjectiveID (Utilities|Struct|BreakF_ObjectiveDetails _array_element)))
        (Utilities|Map|Add (Variables|Default|GetCurrentObjectiveProgress) (.ObjectiveID (Utilities|Struct|BreakF_ObjectiveDetails _array_element)) 0)))))

(fn GetObjectiveDatabyID
  (params (ObjectiveID :type String))
  ;[0.15 0.15 0.15 0.5] Gets objective data by looping through the Id's in the objectives array
  (for _array_element (.Objectives (Utilities|Struct|BreakF_StageDetails (Variables|Default|GetCurrentStageDetails)))
    (if (Utilities|Enum|Equal(Enum) (.ObjectiveID (Utilities|Struct|BreakF_ObjectiveDetails _array_element)) ObjectiveID)
      (return _array_element))))

(fn IsObjectiveComplete
  (params (ObjectiveID :type String))
  (bind _array_element (CallFunction|GetObjectiveDatabyID ObjectiveID))
  (bind (_objectivename _objectivedesc _objectivetype _objectiveid _quantity) (Utilities|Struct|BreakF_ObjectiveDetails _array_element))
  (if (>= (.Value (Utilities|Map|Find (Variables|Default|GetCurrentObjectiveProgress) ObjectiveID)) _quantity)
    (bind _returnvalue (UserInterface|CreateWidget "/Game/QuestSystem/UI/WBP_QuestNotif.WBP_QuestNotif_C" 0 _objectivedesc))
    (UserInterface|Viewport|AddtoViewport _returnvalue 0)
    (bind _return (CallFunction|IsAllObjectivesComplete))
    (if _return
      (bind _result (Math|Integer|IncrementInt (Variables|Default|GetCurrentStage))
        (:%20%20
          (if (Utilities|Array|IsValidIndex (.Stages (Utilities|Struct|BreakF_QuestDetails (Variables|Default|GetQuestDetails))) _result)
            (CallFunction|GetQuestDetails)
            (else
              (bind _output_get (Variables|Default|SetIsCompleted true))
              (bind _timeelapsed (Class|BPIGameMode|StopQuestTimer(Message) (Game|GetGameMode)))
              (Class|BPIPlayerInformation|SetIsQuestCompleted(Message) (Game|GetPlayerCharacter 0) _output_get (Variables|Default|GetCompletion%20Time) _timeelapsed))))))))

(fn IsAllObjectivesComplete
  (for _array_element (.Objectives (Utilities|Struct|BreakF_StageDetails (Variables|Default|GetCurrentStageDetails)))
    (if (not (>= (.Value (Utilities|Map|Find (Variables|Default|GetCurrentObjectiveProgress) (.ObjectiveID (Utilities|Struct|BreakF_ObjectiveDetails _array_element)))) (.Quantity (Utilities|Struct|BreakF_ObjectiveDetails (CallFunction|GetObjectiveDatabyID (.ObjectiveID (Utilities|Struct|BreakF_ObjectiveDetails _array_element)))))))
      (bind _output_get (LocalVariables|SetLocal_AllComplete false))
      (return _output_get)))
  (return (LocalVariables|GetLocal_AllComplete)))